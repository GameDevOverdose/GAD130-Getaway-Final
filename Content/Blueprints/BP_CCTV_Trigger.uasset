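; CCTV trigger volume that moves a linked door when a shooter character enters or leaves while the camera system is enabled.
; A timeline lerps the door's height between ClosedZ and OpenedZ, reversing on entry and playing forward on exit and at BeginPlay.
; Paired DoOnce gates play the door sound on each move while CCTV is enabled.
; Tick keeps driving the timeline forward whenever CCTV is disabled.
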(event `self.BoxTrigger.OnComponentBeginOverlap`
  (params (OverlappedComponent :type "PrimitiveComponent Object Reference") (OtherActor :type "Actor Object Reference") (OtherComp :type "PrimitiveComponent Object Reference") (OtherBodyIndex :type Integer) (bFromSweep :type Boolean) (SweepResult :type "HitResult Structure (by ref)"))
  (bind _door (`self.Door`))
  (bind (_returnvalue_x _returnvalue_y) (`KismetMathLibrary.BreakVector` (`self.K2_GetActorLocation` _door)))
  ; CCTV Door Behavior
  (`|ExecutionSequence`
    (:`then_0`
      (bind _output_get (set `self.Other Actor` OtherActor))
      (bind _asbp_shooter_character (cast `/Game/Variant_Shooter/Blueprints/BP_ShooterCharacter` _output_get))
      (if (and (`self.CCTVEnabled`) (`KismetSystemLibrary.IsValid` _asbp_shooter_character))
        (bind (_direction _value) (`Timeline|Timeline` :!via `Reverse` :!label _label)
          (:`Update`
            (`self.K2_SetActorRelativeLocation` _door (`KismetMathLibrary.MakeVector` _returnvalue_x _returnvalue_y (`KismetMathLibrary.Lerp` (`self.ClosedZ`) (`self.OpenedZ`) _value)) false false)))))
    (:`then_1`
      (`/Engine/EditorBlueprintResources/StandardMacros.DoOnce` false :!label _label_2
        (:`Completed`
          (if (`self.CCTVEnabled`) :!label _label_3
            (`GameplayStatics.SpawnSoundAttached` "/Game/Audio/Door_Open_Fast.Door_Open_Fast" (`Actor.RootComponent` (`self.Door`)) "None" (0.0 0.0 0.0) (struct) "KeepRelativeOffset" false (`self.DoorOpenVolume`) 1.0 0.0 null null)))))
    (:`then_2`
      (goto _label_4 :!via `Reset`))))

(event `self.ReceiveBeginPlay`
  ; CCTV Door Behavior
  (`|ExecutionSequence`
    (:`then_0`
      (goto _label))
    (:`then_1`
      (set `self.CCTVEnabled` true))))

(event `self.ReceiveTick`
  (params (DeltaSeconds :type "Float (single-precision)"))
  ; CCTV Door Behavior
  (if (not (`self.CCTVEnabled`))
    (goto _label)))

(event `self.BoxTrigger.OnComponentEndOverlap`
  (params (OverlappedComponent :type "PrimitiveComponent Object Reference") (OtherActor :type "Actor Object Reference") (OtherComp :type "PrimitiveComponent Object Reference") (OtherBodyIndex :type Integer))
  ; CCTV Door Behavior
  (`|ExecutionSequence`
    (:`then_0`
      (bind _output_get (set `self.Other Actor` OtherActor))
      (cast `/Game/Variant_Shooter/Blueprints/BP_ShooterCharacter` _output_get)
      (goto _label))
    (:`then_1`
      (goto _label_2 :!via `Reset`))
    (:`then_2`
      (`/Engine/EditorBlueprintResources/StandardMacros.DoOnce` false :!label _label_4
        (:`Completed`
          (goto _label_3))))))

(fn `UserConstructionScript`)