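; Interactable electrical panel that powers up the area when the player presses E within its trigger while HasFuse is set.
; The trigger overlap toggles input and shows a prompt; HasFuse starts false and is not granted here.
; A one-shot sequence destroys a linked door, swaps visibility of tagged actors, and uses staggered delays for generator sound, lights and music.
; Music starts by setting ConditionSatisfied on tagged BP_SoundPlayer actors.
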(event `self.BoxTrigger.OnComponentBeginOverlap`
  (params (OverlappedComponent :type "PrimitiveComponent Object Reference") (OtherActor :type "Actor Object Reference") (OtherComp :type "PrimitiveComponent Object Reference") (OtherBodyIndex :type Integer) (bFromSweep :type Boolean) (SweepResult :type "HitResult Structure (by ref)"))
  ; Interaction Logic
  (cast `/Game/Variant_Shooter/Blueprints/BP_ShooterCharacter` OtherActor)
  (`self.EnableInput` (`GameplayStatics.GetPlayerController` 0))
  (`KismetSystemLibrary.PrintString` "PRESS E TO INTERACT" true true (struct :`R` 1.0 :`G` 1.0 :`B` 1.0 :`A` 1.0) 2.0 "Interact"))

(event `Key|E`
  (params (Key :type "Key Structure"))
  ; Check & Execute
  (:`Pressed`
    (if (`self.HasFuse`)
      (`|ExecutionSequence`
        (:`then_0`
          (`/Engine/EditorBlueprintResources/StandardMacros.DoOnce` false
            (:`Completed`
              (`KismetSystemLibrary.PrintString` "FUSE PLACED" true true (struct :`R` 0.577581 :`A` 1.0))
              (`|ExecutionSequence`
                (:`then_0`
                  (`self.K2_DestroyActor` (`self.DoorToDisable`))
                  (bind _outactors (`GameplayStatics.GetAllActorsWithTag` "DisableOnFusePlace"))
                  (for _array_element _outactors
                    (`self.SetActorHiddenInGame` _array_element true)))
                (:`then_1`
                  (`KismetSystemLibrary.Delay` (`self.GeneratorSoundDelay`))
                  (`GameplayStatics.SpawnSound2D` "/Game/Audio/Generator.Generator" 1.0 1.0 0.0 null))
                (:`then_2`
                  (`KismetSystemLibrary.Delay` (`self.LightsEnableDelay`))
                  (bind _outactors_2 (`GameplayStatics.GetAllActorsWithTag` "EnableOnFusePlace"))
                  (for _array_element_2 _outactors_2
                    (`self.SetActorHiddenInGame` _array_element_2 false)))
                (:`then_3`
                  (`KismetSystemLibrary.Delay` (`self.MusicDelay`))
                  (bind _outactors_3 (`GameplayStatics.GetAllActorsWithTag` "MusicSpeaker"))
                  (for _array_element_3 _outactors_3
                    (bind _asbp_sound_player (cast `/Game/Blueprints/BP_SoundPlayer` _array_element_3))
                    (set `/Game/Blueprints/BP_SoundPlayer.ConditionSatisfied` true _asbp_sound_player)))))))
        (:`then_1`
          (set `self.FusePlaced` true)))
      (else
        (`KismetSystemLibrary.PrintString` "FUSE MISSING" true true (struct :`R` 1.0 :`G` 1.0 :`B` 1.0 :`A` 1.0))))))

(event `self.ReceiveBeginPlay`
  ; Start Sequence
  (set `self.HasFuse` false)
  (bind _outactors (`GameplayStatics.GetAllActorsWithTag` "EnableOnFusePlace"))
  (for _array_element _outactors
    (`self.SetActorHiddenInGame` _array_element true)))

(event `self.BoxTrigger.OnComponentEndOverlap`
  (params (OverlappedComponent :type "PrimitiveComponent Object Reference") (OtherActor :type "Actor Object Reference") (OtherComp :type "PrimitiveComponent Object Reference") (OtherBodyIndex :type Integer))
  ; Interaction Logic
  (`self.DisableInput` (`GameplayStatics.GetPlayerController` 0)))

(fn `UserConstructionScript`)