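; BP_Gate is a gate actor that slides vertically between closed and opened Z heights, with attached open and close sounds.
; The OpenGate event acts as a toggle through a FlipFlop, alternately playing and reversing a Timeline; BeginPlay fires the same toggle when OpenAtStart is set.
; The Timeline lerps relative Z while reusing the actor's current world X and Y.
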(event `self.ReceiveBeginPlay`
  (bind (_returnvalue_x _returnvalue_y) (`KismetMathLibrary.BreakVector` (`self.K2_GetActorLocation`)))
  (if (`self.OpenAtStart`)
    (`/Engine/EditorBlueprintResources/StandardMacros.FlipFlop` :!label _label
      (:`A`
        (`|ExecutionSequence`
          (:`then_0`
            (`GameplayStatics.SpawnSoundAttached` (`self.OpenSound`) (`self.DefaultSceneRoot`) "None" (0.0 0.0 0.0) (struct) "KeepRelativeOffset" false (`self.OpenSoundVolume`) 1.0 0.0 "/Game/Audio/SpeakerMusic.SpeakerMusic" null))
          (:`then_1`
            (bind (_direction _value) (`Timeline|Timeline` :!label _label_2)
              (:`Update`
                (`self.K2_SetActorRelativeLocation` (`KismetMathLibrary.MakeVector` _returnvalue_x _returnvalue_y (`KismetMathLibrary.Lerp` (`self.ClosedZ`) (`self.OpenedZ`) _value))))))))
      (:`B`
        (`|ExecutionSequence`
          (:`then_0`
            (goto _label_2 :!via `Reverse`))
          (:`then_1`
            (`GameplayStatics.SpawnSoundAttached` (`self.CloseSound`) (`self.DefaultSceneRoot`) "None" (0.0 0.0 0.0) (struct) "KeepRelativeOffset" false (`self.CloseSoundVolume`) 1.0 0.0 "/Game/Audio/SpeakerMusic.SpeakerMusic" null)))))))

(event `OpenGate`
  (goto _label))

(fn `UserConstructionScript`)