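; BP_EndingMusic is a trigger box that plays the ending sequence, with music, a cut to black and a title.
; Its first overlap passes a DoOnce before the Player tag check, so another actor entering first uses up the trigger.
; For the player, it plays a 2D track, then after separate delays shows existing Black widgets and adds a new ending title widget to the viewport.
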(event `self.Box.OnComponentBeginOverlap`
  (params (OverlappedComponent :type "PrimitiveComponent Object Reference") (OtherActor :type "Actor Object Reference") (OtherComp :type "PrimitiveComponent Object Reference") (OtherBodyIndex :type Integer) (bFromSweep :type Boolean) (SweepResult :type "HitResult Structure (by ref)"))
  (`/Engine/EditorBlueprintResources/StandardMacros.DoOnce` false
    (:`Completed`
      (if (`self.ActorHasTag` OtherActor "Player")
        (`GameplayStatics.SpawnSound2D` "/Game/Audio/The_Red_Capes_Are_Coming.The_Red_Capes_Are_Coming" (`self.MusicVolume`) 1.0 0.0 null)
        (`|ExecutionSequence`
          (:`then_0`
            (`KismetSystemLibrary.Delay` (`self.CutToBlackDelay`))
            (bind _foundwidgets (`WidgetBlueprintLibrary.GetAllWidgetsOfClass` "/Game/Black.Black_C"))
            (`Widget.SetVisibility` _foundwidgets "Visible"))
          (:`then_1`
            (`KismetSystemLibrary.Delay` (`self.TitleRevealDelay`))
            (bind _returnvalue (`|CreateWidget` "/Game/EndingTitle.EndingTitle_C"))
            (`/Game/EndingTitle.Split` _returnvalue)
            (`UserWidget.AddToViewport` _returnvalue 0)))))))

(fn `UserConstructionScript`)