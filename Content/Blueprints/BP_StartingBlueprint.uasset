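; Opening-sequence Blueprint that plays a timed audio and title intro when play begins.
; A Sequence starts looping-capable room ambience, shows a Black widget, then uses separate delays to play glass breaking, swap to the OpeningTitle widget, and finally hide the title.
; Widgets are hidden through class lookups rather than stored references.
; A BoxTrigger overlap filters for BP_ShooterCharacter into a DoOnce with nothing connected after it.
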(event `self.ReceiveBeginPlay`
  (`|ExecutionSequence`
    (:`then_0`
      (`GameplayStatics.SpawnSound2D` "/Game/Audio/Empty_Room_Ambient_Noise_Sound_Effect.Empty_Room_Ambient_Noise_Sound_Effect" (`self.AmbienceVolume`) 1.0 0.0 null false false))
    (:`then_1`
      (bind _returnvalue (`|CreateWidget` "/Game/Black.Black_C"))
      (`UserWidget.AddToViewport` _returnvalue 0)
      (`KismetSystemLibrary.Delay` (`self.GlassBreakSoundDelay`))
      (`GameplayStatics.SpawnSound2D` "/Game/Audio/Glass_Breaking_Sound_Effect.Glass_Breaking_Sound_Effect" (`self.GlassBreakSoundVolume`) 1.0 0.0 null false false))
    (:`then_2`
      (`KismetSystemLibrary.Delay` (`self.Title Reveal Delay`))
      (bind _returnvalue_2 (`|CreateWidget` "/Game/OpeningTitle.OpeningTitle_C"))
      (`UserWidget.AddToViewport` _returnvalue_2 0)
      (bind _foundwidgets (`WidgetBlueprintLibrary.GetAllWidgetsOfClass` "/Game/Black.Black_C"))
      (`Widget.SetVisibility` _foundwidgets "Hidden"))
    (:`then_3`
      (`KismetSystemLibrary.Delay` (`self.GameAppearDelay`))
      (bind _foundwidgets_2 (`WidgetBlueprintLibrary.GetAllWidgetsOfClass` "/Game/OpeningTitle.OpeningTitle_C"))
      (`Widget.SetVisibility` _foundwidgets_2 "Hidden"))))

(event `self.BoxTrigger.OnComponentBeginOverlap`
  (params (OverlappedComponent :type "PrimitiveComponent Object Reference") (OtherActor :type "Actor Object Reference") (OtherComp :type "PrimitiveComponent Object Reference") (OtherBodyIndex :type Integer) (bFromSweep :type Boolean) (SweepResult :type "HitResult Structure (by ref)"))
  (cast `/Game/Variant_Shooter/Blueprints/BP_ShooterCharacter` OtherActor)
  (`/Engine/EditorBlueprintResources/StandardMacros.DoOnce` false))

(fn `UserConstructionScript`)